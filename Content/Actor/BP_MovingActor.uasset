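; Moving actor that oscillates back and forth along the world X axis around its starting position while Onoff is true.
; The first Tick caches the starting X in Move, then each Tick steps X by Multiplaier without delta-time scaling.
; When the next step would pass Move plus or minus Max, it flips IsLocationIncerese instead of moving.
; An alternative Timeline-driven version is present but disconnected and never runs.
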(event `self.ReceiveBeginPlay`)

(event `self.ReceiveTick`
  (params (DeltaSeconds :type "Float (single-precision)"))
  (bind (_returnvalue_x _returnvalue_y _returnvalue_z) (`KismetMathLibrary.BreakVector` (`self.K2_GetActorLocation`)))
  (bind _multiplaier (`self.Multiplaier`))
  (bind _max (`self.Max`))
  (bind _returnvalue (+ (`self.Move`) (select `bool` (`self.isLocationIncerese`) :`false` (* _max -1.0) :`true` _max)))
  (bind _returnvalue_2 (+ (.x (`self.K2_GetActorLocation`)) (select `bool` (`self.isLocationIncerese`) :`false` (* -1.0 _multiplaier) :`true` _multiplaier)))
  ;[1 1 1] 반복운동
  (`|ExecutionSequence`
    (:`then_0`
      (`/Engine/EditorBlueprintResources/StandardMacros.DoOnce` false
        (:`Completed`
          (bind _output_get (set `self.location` (`self.K2_GetActorLocation`)))
          (set `self.Move` (.x _output_get)))))
    (:`then_1`
      (if (`self.on/off`)
        (if (select `bool` (`self.isLocationIncerese`) :`false` (< _returnvalue_2 _returnvalue) :`true` (> _returnvalue_2 _returnvalue))
          (set `self.isLocationIncerese` (not (`self.isLocationIncerese`)))
          (else
            (`self.K2_SetActorLocation` (`KismetMathLibrary.MakeVector` _returnvalue_2 _returnvalue_y _returnvalue_z))))))))

(fn `UserConstructionScript`)