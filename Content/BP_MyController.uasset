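; BP_MyController is a player controller that drives the possessed pawn and lets the player switch bodies with another pawn.
; It adds an Enhanced Input mapping context at BeginPlay and caches the possessed BP_BasePawn.
; Move input follows control rotation, scaled by that pawn's MovementMultiplier, while look input adds yaw and pitch.
; Completing Interact possesses the pawn's OverlappedPawn if valid; the jump handler is empty.
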(event `self.ReceiveBeginPlay`
  (bind _returnvalue (pcsubsystem `EnhancedInputLocalPlayerSubsystem` self))
  ;[1 1 1] 매핑 불러오기
  (`/Engine/EditorBlueprintResources/StandardMacros.IsValid` _returnvalue
    (:`Is Valid`
      (`EnhancedInputSubsystemInterface.AddMappingContext` _returnvalue "/Game/Input/IMC_MyAction.IMC_MyAction" 0 (struct)))))

(event `self.ReceivePossess`
  (params (PossessedPawn :type "Pawn Object Reference"))
  (bind _asbp_base_pawn (cast `/Game/Actor/BP_BasePawn` PossessedPawn)
    (:`then`
      (set `self.Possesed BasePawn` _asbp_base_pawn))
    (:`CastFailed`
      (set `self.Possesed BasePawn` null))))

(event `EnhancedInput|/Game/Input/IA_MyMove`
  (params (ActionValue :type "Vector2D Structure") (ElapsedSeconds :type "Float (double-precision)") (TriggeredSeconds :type "Float (double-precision)") (InputAction :type "InputAction Object Reference" :default "/Game/Input/IA_MyMove.IA_MyMove"))
  (bind (_returnvalue_roll _returnvalue_pitch _returnvalue_yaw) (`KismetMathLibrary.BreakRotator` (`self.GetControlRotation`)))
  (bind (_returnvalue_roll_2 _returnvalue_pitch_2 _returnvalue_yaw_2) (`KismetMathLibrary.BreakRotator` (`self.GetControlRotation`)))
  ;[1 1 1] 움직이기
  (:`Triggered`
    (`Pawn.AddMovementInput` (`self.K2_GetPawn`) (* (* ActionValue_X (`/Game/Actor/BP_BasePawn.MovementMultiplier` (`self.Possesed BasePawn`))) (`KismetMathLibrary.GetRightVector` (`KismetMathLibrary.MakeRotator` _returnvalue_roll_2 0.0 _returnvalue_yaw_2))) 1.0 false)
    (`Pawn.AddMovementInput` (`self.K2_GetPawn`) (* (* ActionValue_Y (`/Game/Actor/BP_BasePawn.MovementMultiplier` (`self.Possesed BasePawn`))) (`KismetMathLibrary.GetForwardVector` (`KismetMathLibrary.MakeRotator` 0.0 0.0 _returnvalue_yaw))) 1.0 false)))

(event `EnhancedInput|/Game/Input/IA_MyLook`
  (params (ActionValue :type "Vector2D Structure") (ElapsedSeconds :type "Float (double-precision)") (TriggeredSeconds :type "Float (double-precision)") (InputAction :type "InputAction Object Reference" :default "/Game/Input/IA_MyLook.IA_MyLook"))
  ;[1 1 1] 시점변경
  (:`Triggered`
    (`self.AddYawInput` ActionValue_X)
    (`self.AddPitchInput` ActionValue_Y)))

(event `EnhancedInput|/Game/Input/IA_MyJump`
  (params (ActionValue :type Boolean) (ElapsedSeconds :type "Float (double-precision)") (TriggeredSeconds :type "Float (double-precision)") (InputAction :type "InputAction Object Reference" :default "/Game/Input/IA_MyJump.IA_MyJump")))

(event `EnhancedInput|/Game/Input/IA_Interact`
  (params (ActionValue :type Boolean) (ElapsedSeconds :type "Float (double-precision)") (TriggeredSeconds :type "Float (double-precision)") (InputAction :type "InputAction Object Reference" :default "/Game/Input/IA_Interact.IA_Interact"))
  (bind _overlappedpawn (`/Game/Actor/BP_BasePawn.OverlappedPawn` (`self.Possesed BasePawn`)))
  (:`Completed`
    (`/Engine/EditorBlueprintResources/StandardMacros.IsValid` _overlappedpawn
      (:`Is Valid`
        (`self.Possess` _overlappedpawn)))))

(fn `UserConstructionScript`)